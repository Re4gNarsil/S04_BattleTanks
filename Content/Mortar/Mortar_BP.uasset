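; Mortar Blueprint that sets up a dome-and-barrel aimed weapon with a health bar and damage effects.
; On BeginPlay it initialises its aiming component with the barrel and dome, then passes itself to the Healthbar_BP widget as both tank and mortar reference.
; HeavilyDamaged activates the ImpactBlast effect and RemoveFlames deactivates it.
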(event `self.ReceiveBeginPlay`
  (`TankAimingComponent.InitialiseAiming` (`self.TankAiming_0`) (`self.MortarBarrel`) (`self.MortarDome`))
  (bind _ashealthbar_bp (cast `/Game/UI/Healthbar_BP` (`WidgetComponent.GetUserWidgetObject` (`self.Widget_0`))))
  (set `/Game/UI/Healthbar_BP.OurTankRef` self _ashealthbar_bp)
  (set `/Game/UI/Healthbar_BP.MortarBPRef` self _ashealthbar_bp))

(event `HeavilyDamaged`
  (`ActorComponent.Activate` (`self.ImpactBlast`) false))

(event `RemoveFlames`
  (`ActorComponent.Deactivate` (`self.ImpactBlast`)))

(fn `UserConstructionScript`)